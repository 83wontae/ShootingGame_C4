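; BP_RandomSpawnWeapon is a spawner that scatters a handful of randomly chosen weapons around itself when play begins.
; On BeginPlay it reads the DT_Weapon row names, then loops to spawn BP_MachineGun actors at random navigable points within a fixed radius of its location.
; Each spawn receives a random row name as WeaponName, so one Blueprint class serves every table entry and repeats are possible.
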(event `self.ReceiveBeginPlay`
  (bind _outrownames (`DataTableFunctionLibrary.GetDataTableRowNames` "/Game/Shooting/Data/DT_Weapon.DT_Weapon"))
  (set `self.Out Row Names` _outrownames)
  (for _ (range 4)
    (`|SpawnActorFromClass` "/Game/Shooting/Blueprints/BP_MachineGun.BP_MachineGun_C" (`KismetMathLibrary.MakeTransform` (`NavigationSystemV1.K2_GetRandomLocationInNavigableRadius` (`self.K2_GetActorLocation`) 500.0 null null)) "Undefined" "OverrideRootScale" null (`|GetArrayItem` (`self.Out Row Names`) (`KismetMathLibrary.RandomInteger` (`KismetArrayLibrary.Array_Length` (`self.Out Row Names`)))) null)))

(fn `UserConstructionScript`)