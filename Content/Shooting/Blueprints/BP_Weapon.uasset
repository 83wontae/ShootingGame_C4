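; Rifle weapon actor that a character attaches to a mesh socket and fires, or detaches as a physics object.
; PullTrigger plays the character's shoot montage while ammo remains, decrementing the count and updating BP_ShootingHud.
; DoShoot is separate from the trigger and ammo logic, playing audio and a muzzle effect, then line-tracing from the player camera.
; Only destructible components take damage and impulse from hits.
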(fn `AttachToChar`
  (params (Character :type "Character Object Reference"))
  (returns (Result :type Boolean) (Actor :type "Actor Object Reference"))
  (bind _staticmesh (`self.StaticMesh`))
  (bind _output_get (set `self.OwnChar` Character))
  (bind _asbp_shooting_hud (cast `/Game/Shooting/GameMode/BP_ShootingHud` (`PlayerController.GetHUD` (`GameplayStatics.GetPlayerController` 0))))
  (`/Game/Shooting/GameMode/BP_ShootingHud.SetAmmoText` _asbp_shooting_hud (`self.Ammo`))
  (`PrimitiveComponent.SetSimulatePhysics` _staticmesh false)
  (`PrimitiveComponent.SetCollisionEnabled` _staticmesh "NoCollision")
  (bind _returnvalue (`SceneComponent.K2_AttachToComponent` _staticmesh (`Character.Mesh` _output_get) (`self.Socket Name`) "SnapToTarget" "SnapToTarget" "KeepWorld" true))
  (return _returnvalue self))

(fn `CheckShootable`
  (returns (Shootable :type Boolean))
  (`/Engine/EditorBlueprintResources/StandardMacros.IsValid` (`self.OwnChar`)
    (:`Is Valid`
      (if (> (`self.Ammo`) 0)
        (return true)
        (else
          (return false))))
    (:`Is Not Valid`
      (return false))))

(fn `DetachToChar`
  (params (Character :type "Character Object Reference"))
  (returns (Result :type Boolean))
  (bind _staticmesh (`self.StaticMesh`))
  (`PrimitiveComponent.SetCollisionEnabled` _staticmesh "QueryAndPhysics")
  (`PrimitiveComponent.SetSimulatePhysics` _staticmesh true)
  (`SceneComponent.K2_DetachFromComponent` _staticmesh "KeepWorld" "KeepWorld" "KeepWorld" true)
  (return true))

(fn `DoShoot`
  (params (Character :type "Character Object Reference"))
  (returns (Result :type Boolean))
  (bind _returnvalue (`GameplayStatics.GetPlayerCameraManager` 0))
  (bind _returnvalue_2 (`self.K2_GetActorLocation` _returnvalue))
  (`AudioComponent.Play` (`self.Audio`) 0.0)
  (`GameplayStatics.SpawnEmitterAtLocation` "/Game/StarterContent/Particles/P_Explosion.P_Explosion" (`SceneComponent.GetSocketLocation` (`self.StaticMesh`) "Muzzle") (struct) (0.1 0.1 0.1))
  (bind (_outhit _returnvalue_3) (`KismetSystemLibrary.LineTraceSingleForObjects` :`Start` (+ _returnvalue_2 (* (`self.GetActorForwardVector` _returnvalue) 300.0)) :`End` (+ _returnvalue_2 (* (`self.GetActorForwardVector` _returnvalue) 2000.0)) :`ObjectTypes` (`|MakeArray` "ObjectTypeQuery1" "ObjectTypeQuery2" "ObjectTypeQuery3" "ObjectTypeQuery4" "ObjectTypeQuery6" :!type "EObjectTypeQuery Enum") :`DrawDebugType` "ForDuration"))
  (if _returnvalue_3
    (bind (_bblockinghit _binitialoverlap _time _distance _location _impactpoint _normal _impactnormal _physmat _hitactor _hitcomponent) (`GameplayStatics.BreakHitResult` _outhit))
    (bind _asdestructible_component (cast `DestructibleComponent` _hitcomponent))
    (`DestructibleComponent.ApplyDamage` _asdestructible_component 100.0 _impactpoint (`self.GetActorForwardVector` (`GameplayStatics.GetPlayerCameraManager` 0)) 100000.0)
    (return true)))

(fn `PlayShootMontage`
  (bind _ownchar (`self.OwnChar`))
  (bind _shootable (`self.CheckShootable`))
  (if _shootable
    (`/Engine/EditorBlueprintResources/StandardMacros.IsValid` _ownchar
      (:`Is Valid`
        (`AnimInstance.Montage_Play` (`SkeletalMeshComponent.GetAnimInstance` (`Character.Mesh` _ownchar)) "/Game/Mannequin/Animations/InPlace/Rifle_ShootOnce_Montage.Rifle_ShootOnce_Montage" 1.0 "MontageLength" 0.0 true)
        (bind _result (`/Engine/EditorBlueprintResources/StandardMacros.DecrementInt` (`self.Ammo`))
          (:`  `
            (bind _asbp_shooting_hud (cast `/Game/Shooting/GameMode/BP_ShootingHud` (`PlayerController.GetHUD` (`GameplayStatics.GetPlayerController` 0))))
            (`/Game/Shooting/GameMode/BP_ShootingHud.SetAmmoText` _asbp_shooting_hud _result)))))))

(fn `PullTrigger`
  (params (Character :type "Character Object Reference"))
  (returns (Result :type Boolean))
  (`self.PlayShootMontage`)
  (return true))

(fn `ReleaseTrigger`
  (params (Character :type "Character Object Reference"))
  (returns (Result :type Boolean))
  (return false))

(fn `UserConstructionScript`)