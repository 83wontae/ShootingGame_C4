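; BP_MoveRightLeft is a Blueprint that slides its Cube back and forth along relative X between zero and a fixed limit.
; Pressing P toggles a looping function-name timer that calls UpdateMoveRightLeft at short intervals, so motion needs no Tick.
; Each update offsets the Cube by Speed scaled to the timer interval and flips IsRight at either bound to reverse direction.
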(event `self.ReceiveBeginPlay`)

(event `/Game/Shooting/Data/BPI_MoveActor.PressP`
  (if (`KismetSystemLibrary.K2_TimerExists` null "UpdateMoveRightLeft")
    (`KismetSystemLibrary.K2_ClearTimer` null "UpdateMoveRightLeft")
    (else
      (`KismetSystemLibrary.K2_SetTimer` null "UpdateMoveRightLeft" 0.01 true))))

(fn `UpdateMoveRightLeft`
  (bind _returnvalue (* (`self.Speed`) 0.01))
  (bind _relativelocation_x (`KismetMathLibrary.BreakVector` (`SceneComponent.RelativeLocation` (`self.Cube`))))
  (bind _relativelocation_x_2 (`KismetMathLibrary.BreakVector` (`SceneComponent.RelativeLocation` (`self.Cube`))))
  (if (`self.IsRight`)
    (`SceneComponent.K2_AddRelativeLocation` (`self.Cube`) (`KismetMathLibrary.MakeVector` _returnvalue) false false)
    (if (> _relativelocation_x_2 500.0)
      (set `self.IsRight` false))
    (else
      (bind _result (`/Engine/EditorBlueprintResources/StandardMacros.NegateFloat` _returnvalue)
        (:`  `
          (`SceneComponent.K2_AddRelativeLocation` (`self.Cube`) (`KismetMathLibrary.MakeVector` _result) false false)
          (if (<= _relativelocation_x 0.0)
            (set `self.IsRight` true)))))))

(fn `UserConstructionScript`)