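; BP_ShootingPlayerState is the player state for the shooting game mode, holding a player's Hp.
; AddDamage subtracts damage from Hp without clamping.
; The Hp RepNotify prints a debug message and, only when this state belongs to the first local player controller, fires the UpdateHp dispatcher with current Hp and a hardcoded maximum.
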(fn `AddDamage`
  (params (Damage :type "Float (double-precision)"))
  (set `self.Hp` (- (`self.Hp`) Damage)))

(fn `OnRep_Hp`
  (`KismetSystemLibrary.PrintString` (`KismetStringLibrary.Concat_StrStr` "OnRepHp CurHP - " (`KismetStringLibrary.Conv_DoubleToString` (`self.Hp`))) true true (struct :`G` 0.66 :`B` 1.0 :`A` 1.0) 20.0)
  (if (== (`Controller.PlayerState` (`GameplayStatics.GetPlayerController` 0)) self)
    (`self.EventDispatcher_UpdateHp` (`self.Hp`) 100.0)))

(fn `UserConstructionScript`)