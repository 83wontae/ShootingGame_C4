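; Shooting game HUD Blueprint that creates and displays the shooting HUD widget for ammo and health.
; On BeginPlay it adds the widget to the viewport and binds to the UpdateHp dispatcher on player 0's BP_ShootingPlayerState, printing an error if the cast fails.
; SetAmmoText and SetHp act as pass-throughs that forward ammo and current/max HP values to the widget.
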(event `self.ReceiveBeginPlay`
  (bind _returnvalue (`|CreateWidget` "/Game/Shooting/Widget/ShootingHudWidget.ShootingHudWidget_C"))
  (bind _output_get (set `self.HudWidget` _returnvalue))
  (`UserWidget.AddToViewport` _output_get 0)
  (bind _asbp_shooting_player_state (cast `/Game/Shooting/GameMode/BP_ShootingPlayerState` (`Controller.PlayerState` (`GameplayStatics.GetPlayerController` 0)))
    (:`then`
      (add `/Game/Shooting/GameMode/BP_ShootingPlayerState.EventDispatcher_UpdateHp` _asbp_shooting_player_state (`|CreateDelegate` :!event `SetHp`)))
    (:`CastFailed`
      (`KismetSystemLibrary.PrintString` "Fail To Cast PlayerState" true true (struct :`R` 1.0 :`A` 1.0) 20.0))))

(fn `SetAmmoText`
  (params (Ammo :type Integer))
  (`/Game/Shooting/Widget/ShootingHudWidget.SetAmmoText` (`self.HudWidget`) Ammo))

(fn `SetHp`
  (params (CurHp :type "Float (double-precision)") (MaxHp :type "Float (double-precision)"))
  (`/Game/Shooting/Widget/ShootingHudWidget.SetHP` (`self.HudWidget`) CurHp MaxHp))

(fn `UserConstructionScript`)